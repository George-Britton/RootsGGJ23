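; BP_Dino is an enemy that starts with a random roll and bonks the player on contact.
; Player range events start and stop its looping-style audio, and Tick fades volume by vertical distance from the player camera relative to DespawnBoxHeight.
; Overlapping the player capsule plays a boing once and calls the player's Bonk.
; Its own Bonk event runs a timeline driving scale and volume, then destroys the actor.
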(event `self.ReceiveBeginPlay`
  (`self.K2_AddActorWorldRotation` (`KismetMathLibrary.MakeRotator` (`KismetMathLibrary.RandomFloatInRange` 0.0 360.0)))
  (bind _returnvalue (`GameplayStatics.GetActorOfClass` "/Script/RootsGGJ23.PlayerRoot"))
  (bind _output_get (set `self.Player` _returnvalue))
  (add `PlayerRoot.OnInRangeOfPlayer` _output_get (delegate `OnInRangeOfPlayer_Event_0`))
  (add `PlayerRoot.OnOutOfRangeOfPlayer` _output_get (delegate `OnOutOfRangeOfPlayer_Event_0`))
  (set `self.AudioDistance` (`PlayerRoot.DespawnBoxHeight` (`self.Player`))))

(event `OnInRangeOfPlayer_Event_0`
  (params (OtherActor :type "Actor Object Reference"))
  (if (== OtherActor self)
    (`AudioComponent.Play` (`self.Audio`) 0.0)))

(event `OnOutOfRangeOfPlayer_Event_0`
  (params (OtherActor :type "Actor Object Reference"))
  (if (== OtherActor self)
    (`AudioComponent.Stop` (`self.Audio`))))

(event `self.ReceiveTick`
  (params (DeltaSeconds :type "Float (single-precision)"))
  (bind (_returnvalue_x _returnvalue_y _returnvalue_z) (`KismetMathLibrary.BreakVector` (`self.K2_GetActorLocation`)))
  (bind _audio (`self.Audio`))
  (bind _player (`self.Player`))
  (bind (_returnvalue_x_2 _returnvalue_y_2 _returnvalue_z_2) (`KismetMathLibrary.BreakVector` (`SceneComponent.K2_GetComponentLocation` (`PlayerRoot.PlayerCamera` _player))))
  (if (and (`AudioComponent.IsPlaying` _audio) (not (`self.Hit`)))
    (bind _output_get (set `AudioComponent.VolumeMultiplier` (`KismetMathLibrary.FClamp` (- 1.0 (/ (`KismetMathLibrary.Vector_Distance` (`KismetMathLibrary.MakeVector` 0.0 0.0 _returnvalue_z) (`KismetMathLibrary.MakeVector` 0.0 0.0 _returnvalue_z_2)) (`PlayerRoot.DespawnBoxHeight` _player))) 0.01) _audio))
    (`AudioComponent.SetVolumeMultiplier` _audio _output_get)))

(event `self.Sphere.OnComponentBeginOverlap`
  (params (OverlappedComponent :type "PrimitiveComponent Object Reference") (OtherActor :type "Actor Object Reference") (OtherComp :type "PrimitiveComponent Object Reference") (OtherBodyIndex :type Integer) (bFromSweep :type Boolean) (SweepResult :type "HitResult Structure (by ref)"))
  (bind _player (`self.Player`))
  (`/Engine/EditorBlueprintResources/StandardMacros.IsValid` _player
    (:`Is Valid`
      (if (and (== OtherComp (`Character.CapsuleComponent` _player)) (not (`self.Hit`)))
        (`GameplayStatics.SpawnSoundAtLocation` "/Game/Audio/BoingCue.BoingCue" (`self.K2_GetActorLocation`) (struct) 1.0 1.0 0.0 null null)
        (set `self.Hit` true)
        (`PlayerRoot.Bonk` (`self.Player`) self)))))

(event `self.Bonk`
  (bind (_direction _newtrack_1) (`Timeline|Timeline_0` :!via `PlayFromStart`)
    (:`Update`
      (`self.SetActorScale3D` (`KismetMathLibrary.Conv_DoubleToVector` _newtrack_1))
      (`AudioComponent.SetVolumeMultiplier` (`self.Audio`) _newtrack_1))
    (:`Finished`
      (`KismetSystemLibrary.Delay` 0.2)
      (`self.K2_DestroyActor`))))

(fn `UserConstructionScript`)