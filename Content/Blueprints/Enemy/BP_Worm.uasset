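; BP_Worm is an enemy that bonks the player once on contact.
; It starts and stops its audio through the player's in-range and out-of-range events, fading volume each tick by distance relative to the player's DespawnBoxHeight.
; The first capsule overlap with the player's capsule plays a boing, calls Bonk on the player, then makes the capsule ignore all collision.
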(event `self.ReceiveBeginPlay`
  (`self.K2_AddActorWorldRotation` (`KismetMathLibrary.MakeRotator` (`KismetMathLibrary.RandomFloat`)))
  (bind _returnvalue (`GameplayStatics.GetActorOfClass` "/Script/RootsGGJ23.PlayerRoot"))
  (bind _output_get (set `self.Player` _returnvalue))
  (add `PlayerRoot.OnInRangeOfPlayer` _output_get (delegate `OnInRangeOfPlayer_Event_0`))
  (add `PlayerRoot.OnOutOfRangeOfPlayer` _output_get (delegate `OnOutOfRangeOfPlayer_Event_0`))
  (set `self.AudioDistance` (`PlayerRoot.DespawnBoxHeight` (`self.Player`))))

(event `OnInRangeOfPlayer_Event_0`
  (params (OtherActor :type "Actor Object Reference"))
  (if (== OtherActor self)
    (`AudioComponent.Play` (`self.Audio`) 0.0)))

(event `OnOutOfRangeOfPlayer_Event_0`
  (params (OtherActor :type "Actor Object Reference"))
  (if (== OtherActor self)
    (`AudioComponent.Stop` (`self.Audio`))))

(event `self.ReceiveTick`
  (params (DeltaSeconds :type "Float (single-precision)"))
  (bind _audio (`self.Audio`))
  (bind _player (`self.Player`))
  (if (`AudioComponent.IsPlaying` _audio)
    (bind _output_get (set `AudioComponent.VolumeMultiplier` (`KismetMathLibrary.FClamp` (- 1.0 (/ (`KismetMathLibrary.Vector_Distance` (`self.K2_GetActorLocation`) (`self.K2_GetActorLocation` _player)) (`PlayerRoot.DespawnBoxHeight` _player))) 0.01) _audio))
    (`AudioComponent.SetVolumeMultiplier` _audio _output_get)))

(event `self.Capsule.OnComponentBeginOverlap`
  (params (OverlappedComponent :type "PrimitiveComponent Object Reference") (OtherActor :type "Actor Object Reference") (OtherComp :type "PrimitiveComponent Object Reference") (OtherBodyIndex :type Integer) (bFromSweep :type Boolean) (SweepResult :type "HitResult Structure (by ref)"))
  (if (and (== OtherComp (`Character.CapsuleComponent` (`self.Player`))) (not (`self.Hit`)))
    (`GameplayStatics.SpawnSoundAtLocation` "/Game/Audio/BoingCue.BoingCue" (`self.K2_GetActorLocation`) (struct) 1.0 1.0 0.0 null null)
    (set `self.Hit` true)
    (`PlayerRoot.Bonk` (`self.Player`) self)
    (`PrimitiveComponent.SetCollisionResponseToAllChannels` (`self.Capsule`) "ECR_Ignore")))

(fn `UserConstructionScript`)