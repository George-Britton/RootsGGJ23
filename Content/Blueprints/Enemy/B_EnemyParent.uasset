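; Parent Blueprint for the Rock, Worm and Mole enemies that the PlayerRoot runs into.
; Construction picks flipbook, sounds and collision setup by enemy type, randomizing rock sprite and rotation and enabling seeking and eating states only for moles.
; The player's range dispatchers start and stop each enemy's audio, while Tick scales volume by player distance over DespawnBoxHeight.
; The first sphere overlap with the player calls Bonk once.
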(event `self.ReceiveBeginPlay`
  (bind _returnvalue (`GameplayStatics.GetActorOfClass` "/Script/RootsGGJ23.PlayerRoot"))
  (bind _output_get (set `self.Player` _returnvalue))
  (add `PlayerRoot.OnInRangeOfPlayer` _output_get (delegate `OnInRangeOfPlayer_Event_0`))
  (add `PlayerRoot.OnOutOfRangeOfPlayer` _output_get (delegate `OnOutOfRangeOfPlayer_Event_0`))
  (set `self.AudioDistance` (`PlayerRoot.DespawnBoxHeight` (`self.Player`))))

(event `OnInRangeOfPlayer_Event_0`
  (params (OtherActor :type "Actor Object Reference"))
  (if (== OtherActor self)
    (`AudioComponent.Play` (`self.Audio`) 0.0)))

(event `OnOutOfRangeOfPlayer_Event_0`
  (params (OtherActor :type "Actor Object Reference"))
  (if (== OtherActor self)
    (`AudioComponent.Stop` (`self.Audio`))))

(event `self.ReceiveTick`
  (params (DeltaSeconds :type "Float (single-precision)"))
  (if (`self.AudioPlaying`)
    (`AudioComponent.SetVolumeMultiplier` (`self.Audio`) (/ (`KismetMathLibrary.Vector_Distance` (`self.K2_GetActorLocation`) (`self.K2_GetActorLocation` (`self.Player`))) (`self.AudioDistance`)))))

(event `self.Sphere1.OnComponentBeginOverlap`
  (params (OverlappedComponent :type "PrimitiveComponent Object Reference") (OtherActor :type "Actor Object Reference") (OtherComp :type "PrimitiveComponent Object Reference") (OtherBodyIndex :type Integer) (bFromSweep :type Boolean) (SweepResult :type "HitResult Structure (by ref)"))
  (bind _asplayer_root (cast `PlayerRoot` OtherActor))
  (if (not (`self.HitPlayer`))
    (`PlayerRoot.Bonk` _asplayer_root self)
    (set `self.HitPlayer` true)))

(fn `CreateEnemyType`
  (`self.SetSound`)
  (switch `/Game/Blueprints/Enemy/E_EnemyType` (`self.EnemyTypes`)
    (:`NewEnumerator0`
      (`PaperFlipbookComponent.SetFlipbook` (`self.EnemyFlipbook`) (`KismetArrayLibrary.Array_Random` (`self.Rocks`)))
      (`self.Set Rock Collision`)
      (return))
    (:`NewEnumerator1`
      (`PaperFlipbookComponent.SetFlipbook` (`self.EnemyFlipbook`) "/Game/Assets/Flipbooks/IMG.IMG")
      (`self.SetCreatureCollision`)
      (return))
    (:`NewEnumerator2`
      ;[1 1 1] Loads in mole underground
      (`PaperFlipbookComponent.SetFlipbook` (`self.EnemyFlipbook`) "/Game/Assets/Flipbooks/MicrosoftTeams-image_Flipbook.MicrosoftTeams-image_Flipbook")
      (`self.SetCreatureCollision`)
      (return))))

(fn `EatRoot`)

(fn `Set Rock Collision`
  (`PrimitiveComponent.SetCollisionProfileName` (`self.Sphere1`) "NoCollision" true)
  (`ActorComponent.SetActive` (`self.MoleSeekingState`) false false)
  (`ActorComponent.SetActive` (`self.MoleEatingState`) false false)
  (`SceneComponent.K2_AddWorldRotation` (`self.EnemyFlipbook`) (`KismetMathLibrary.MakeRotator` (`KismetMathLibrary.RandomFloatInRange` 0.0 360.0)) false false))

(fn `SetCreatureCollision`
  (bind _collisionsound (`self.CollisionSound`))
  (bind _moleseekingstate (`self.MoleSeekingState`))
  (bind _moleeatingstate (`self.MoleEatingState`))
  (switch `/Game/Blueprints/Enemy/E_EnemyType` (`self.EnemyTypes`)
    (:`NewEnumerator0`
      (`AudioComponent.SetSound` _collisionsound "/Game/Audio/BoingCue.BoingCue")
      (`ActorComponent.SetActive` _moleseekingstate false false :!label _label)
      (`ActorComponent.SetActive` _moleeatingstate false false))
    (:`NewEnumerator1`
      (`AudioComponent.SetSound` _collisionsound "/Game/Audio/Wormy_Cue.Wormy_Cue")
      (goto _label))
    (:`NewEnumerator2`
      (`AudioComponent.SetSound` _collisionsound "/Game/Audio/MoleBitingOffRoot.MoleBitingOffRoot")
      (`ActorComponent.SetActive` _moleseekingstate true false)
      (`ActorComponent.SetActive` _moleeatingstate true false))))

(fn `SetSound`
  (bind _audio (`self.Audio`))
  (bind _rocks (`self.Rocks`))
  (switch `/Game/Blueprints/Enemy/E_EnemyType` (`self.EnemyTypes`)
    (:`NewEnumerator0`
      (if (== (`|GetArrayItem` _rocks 2) "/Game/Assets/Flipbooks/Rock_3.Rock_3")
        (`AudioComponent.SetSound` _audio "/Game/Audio/Boulder.Boulder")
        (elif (== (`|GetArrayItem` _rocks 3) "/Game/Assets/Textures/Dino_Skelly_1.Dino_Skelly_1")
          (`AudioComponent.SetSound` _audio "/Game/Audio/Dino_Cue.Dino_Cue")
          (else
            (`AudioComponent.SetSound` _audio (`self.RockSoundOnStart`))))))
    (:`NewEnumerator1`
      (`AudioComponent.SetSound` _audio (`self.WormSoundOnStart`)))
    (:`NewEnumerator2`
      (`AudioComponent.SetSound` _audio (`self.MoleSoundOnStart`))))
  (`AudioComponent.SetVolumeMultiplier` _audio 0.0))

(fn `UserConstructionScript`
  (`self.CreateEnemyType`))