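; Mole enemy that pops into a flipbook animation and bonks the player who touches it.
; Player range events start and stop its audio, and Tick fades volume with distance relative to the player's DespawnBoxHeight.
; A sphere overlap, filtered to the un-hit player capsule, swaps sprite for flipbook and plays the mole sound.
; When the animation finishes, a player still within that distance gets bonked and the sphere ignores further collisions.
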(event `self.ReceiveBeginPlay`
  (bind (_returnvalue_x _returnvalue_y _returnvalue_z) (`KismetMathLibrary.BreakVector` (`self.K2_GetActorLocation`)))
  (bind _paperflipbook (`self.PaperFlipbook`))
  (`PaperFlipbookComponent.Stop` _paperflipbook)
  (`PaperFlipbookComponent.SetLooping` _paperflipbook false)
  (`self.K2_AddActorWorldRotation` (`KismetMathLibrary.MakeRotator` (`KismetMathLibrary.RandomFloat`)))
  (bind _returnvalue (`GameplayStatics.GetActorOfClass` "/Script/RootsGGJ23.PlayerRoot"))
  (bind _output_get (set `self.Player` _returnvalue))
  (add `PlayerRoot.OnInRangeOfPlayer` _output_get (delegate `OnInRangeOfPlayer_Event_0`))
  (add `PlayerRoot.OnOutOfRangeOfPlayer` _output_get (delegate `OnOutOfRangeOfPlayer_Event_0`))
  (set `self.AudioDistance` (`PlayerRoot.DespawnBoxHeight` (`self.Player`)))
  (`self.K2_SetActorLocation` (`KismetMathLibrary.MakeVector` 5.0 _returnvalue_y _returnvalue_z) false true))

(event `OnInRangeOfPlayer_Event_0`
  (params (OtherActor :type "Actor Object Reference"))
  (if (== OtherActor self)
    (`AudioComponent.Play` (`self.Audio`) 0.0)))

(event `OnOutOfRangeOfPlayer_Event_0`
  (params (OtherActor :type "Actor Object Reference"))
  (if (== OtherActor self)
    (`AudioComponent.Stop` (`self.Audio`))))

(event `self.ReceiveTick`
  (params (DeltaSeconds :type "Float (single-precision)"))
  (bind _audio (`self.Audio`))
  (bind _player (`self.Player`))
  (`/Engine/EditorBlueprintResources/StandardMacros.IsValid` (`self.Player`)
    (:`Is Valid`
      _)
    (:`Is Not Valid`
      (bind _returnvalue (`GameplayStatics.GetActorOfClass` "/Script/RootsGGJ23.PlayerRoot"))
      (set `self.Player` _returnvalue)))
  (if (`AudioComponent.IsPlaying` _audio)
    (bind _output_get (set `AudioComponent.VolumeMultiplier` (`KismetMathLibrary.FClamp` (- 1.0 (/ (`KismetMathLibrary.Vector_Distance` (`self.K2_GetActorLocation`) (`self.K2_GetActorLocation` _player)) (`PlayerRoot.DespawnBoxHeight` _player))) 0.01) _audio))
    (`AudioComponent.SetVolumeMultiplier` _audio _output_get)))

(event `self.Sphere.OnComponentBeginOverlap`
  (params (OverlappedComponent :type "PrimitiveComponent Object Reference") (OtherActor :type "Actor Object Reference") (OtherComp :type "PrimitiveComponent Object Reference") (OtherBodyIndex :type Integer) (bFromSweep :type Boolean) (SweepResult :type "HitResult Structure (by ref)"))
  (bind _audio (`self.Audio`))
  (bind _paperflipbook (`self.PaperFlipbook`))
  (`self.CheckIsOverlappingPlayer` OtherComp)
  (`AudioComponent.SetSound` _audio "/Game/Audio/Mole.Mole")
  (`AudioComponent.Play` _audio 0.0)
  (`SceneComponent.SetVisibility` (`self.Sprite`) false false)
  (`SceneComponent.SetVisibility` (`self.PaperFlipbook`) true false)
  (`PaperFlipbookComponent.PlayFromStart` _paperflipbook)
  (add `PaperFlipbookComponent.OnFinishedPlaying` _paperflipbook (delegate `CustomEvent_0`)))

(event `CustomEvent_0`
  (bind _player (`self.Player`))
  (if (< (`KismetMathLibrary.Vector_Distance` (`self.K2_GetActorLocation`) (`self.K2_GetActorLocation` _player)) (`PlayerRoot.DespawnBoxHeight` _player))
    (set `self.Hit` true)
    (`PlayerRoot.Bonk` (`self.Player`) self)
    (`PrimitiveComponent.SetCollisionResponseToAllChannels` (`self.Sphere`) "ECR_Ignore")))

(fn `UserConstructionScript`
  (`PaperFlipbookComponent.SetLooping` (`self.PaperFlipbook`) false))