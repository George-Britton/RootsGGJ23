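; B_parentPickup is a parent pickup actor that grants the player either a speed boost or protection.
; On BeginPlay it destroys itself if the player has both buffs, picks Protection if the player is only fast, and otherwise chooses randomly, setting the matching sprite.
; Overlap with PlayerRoot calls GivePickup for that type, plays the pickup sound and destroys the actor.
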(event `self.ReceiveBeginPlay`
  (bind _returnvalue (`GameplayStatics.GetActorOfClass` "/Script/RootsGGJ23.PlayerRoot"))
  (bind _isfast (`PlayerRoot.IsFast` _returnvalue))
  (if (and _isfast (`PlayerRoot.IsProtected` _returnvalue))
    (`self.K2_DestroyActor`)
    (elif _isfast
      (set `self.PickUpType` "NewEnumerator1" :!label _label)
      (`PaperSpriteComponent.SetSprite` (`self.ObjectSprite`) "/Game/Assets/Sprites/MicrosoftTeams-image__1__Sprite.MicrosoftTeams-image__1__Sprite")
      (elif (`KismetMathLibrary.RandomBool`)
        (set `self.PickUpType` "NewEnumerator0")
        (`PaperSpriteComponent.SetSprite` (`self.ObjectSprite`) "/Game/Assets/Sprites/MicrosoftTeams-image__2__Sprite.MicrosoftTeams-image__2__Sprite")
        (else
          (goto _label))))))

(event `self.Object Collision.OnComponentBeginOverlap`
  (params (OverlappedComponent :type "PrimitiveComponent Object Reference") (OtherActor :type "Actor Object Reference") (OtherComp :type "PrimitiveComponent Object Reference") (OtherBodyIndex :type Integer) (bFromSweep :type Boolean) (SweepResult :type "HitResult Structure (by ref)"))
  (bind _asplayer_root (cast `PlayerRoot` OtherActor))
  (switch `/Game/Blueprints/PickUps/E_PickupType` (`self.PickUpType`)
    (:`NewEnumerator0`
      (`PlayerRoot.GivePickup` _asplayer_root "Zoom"))
    (:`NewEnumerator1`
      (`PlayerRoot.GivePickup` _asplayer_root "Protect")))
  (`self.SoundOnPickup`)
  (`self.K2_DestroyActor`))

(fn `BuffApplication`
  (message `/Game/Blueprints/PickUps/BI_pickup.BuffPickUp` self (`self.Speed Multiplier`) (`self.Shield`)))

(fn `RemoveActor`
  (`self.K2_DestroyActor`))

(fn `SoundOnPickup`
  (`GameplayStatics.SpawnSound2D` (`self.SoundPickup`) 1.0 1.0 0.0 null))

(fn `SoundOnRun`)

(fn `UserConstructionScript`
  (switch `/Game/Blueprints/PickUps/E_PickupType` (`self.PickUpType`)
    (:`NewEnumerator0`
      (`PaperSpriteComponent.SetSprite` (`self.ObjectSprite`) null))
    (:`NewEnumerator1`
      (`PaperSpriteComponent.SetSprite` (`self.ObjectSprite`) null))))