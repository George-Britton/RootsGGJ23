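; Pickup actor that randomly becomes a Spray ("Zoom") or a rarer Drill ("Protect") in its construction script, setting sprite, type and sound.
; When the player's capsule overlaps its sphere, it disables sphere collision, plays the sound, activates a Niagara effect and grants that pickup to PlayerRoot.
; A timeline then animates the actor's scale before destroying it.
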(event `self.ReceiveBeginPlay`
  (bind _returnvalue (`GameplayStatics.GetActorOfClass` "/Script/RootsGGJ23.PlayerRoot"))
  (set `self.Player` _returnvalue))

(event `self.Sphere.OnComponentBeginOverlap`
  (params (OverlappedComponent :type "PrimitiveComponent Object Reference") (OtherActor :type "Actor Object Reference") (OtherComp :type "PrimitiveComponent Object Reference") (OtherBodyIndex :type Integer) (bFromSweep :type Boolean) (SweepResult :type "HitResult Structure (by ref)"))
  (bind _player (`self.Player`))
  (if (== OtherComp (`Character.CapsuleComponent` _player))
    (`GameplayStatics.SpawnSoundAtLocation` (`self.Audio`) (`self.K2_GetActorLocation`) (struct) 1.0 1.0 0.0 null null)
    (`PrimitiveComponent.SetCollisionResponseToAllChannels` (`self.Sphere`) "ECR_Ignore")
    (bind _returnvalue (`AddComponent|NODE_AddNiagaraComponent-0`))
    (`NiagaraComponent.SetAsset` _returnvalue "/Game/ParticleSystems/PS_Pickup.PS_Pickup" true)
    (`ActorComponent.Activate` _returnvalue false)
    (if (`|EnumEquality` (`self.PickupType`) "NewEnumerator0")
      (`PlayerRoot.GivePickup` _player "Zoom")
      (bind (_direction _newtrack_1) (`Timeline|Timeline` :!via `PlayFromStart` :!label _label)
        (:`Update`
          (`self.SetActorScale3D` (`KismetMathLibrary.Conv_DoubleToVector` _newtrack_1)))
        (:`Finished`
          (`self.K2_DestroyActor`)))
      (else
        (`PlayerRoot.GivePickup` _player "Protect")
        (goto _label :!via `PlayFromStart`)))))

(fn `MakeDrill`
  (`PaperSpriteComponent.SetSprite` (`self.PaperSprite`) "/Game/Assets/Sprites/Drill.Drill")
  (set `self.PickupType` "NewEnumerator1")
  (set `self.Audio` "/Game/Audio/Drill.Drill"))

(fn `MakeZoomy`
  (`PaperSpriteComponent.SetSprite` (`self.PaperSprite`) "/Game/Assets/Sprites/Spray.Spray")
  (set `self.PickupType` "NewEnumerator0")
  (set `self.Audio` "/Game/Audio/Spray.Spray"))

(fn `UserConstructionScript`
  (if (`KismetMathLibrary.RandomBoolWithWeight` 0.2)
    (`self.MakeDrill`)
    (else
      (`self.MakeZoomy`))))