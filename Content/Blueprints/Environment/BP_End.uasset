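; BP_End is an environment actor that, when its Make flag is set, populates itself with random enemies and pickups on BeginPlay.
; Random classes from the Spawnable and Pickups arrays spawn at seven enemy and two pickup markers, always ignoring collision.
; Each location comes from GetSpawnLoc, whose graph holds only an unconnected vector with fixed X and random sideways Y offset.
; BeginPlay also caches the PlayerRoot actor as Player.
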(event `self.ReceiveBeginPlay`
  (bind _returnvalue (`GameplayStatics.GetActorOfClass` "/Script/RootsGGJ23.PlayerRoot"))
  (set `self.Player` _returnvalue)
  (if (`self.make`)
    (`|SpawnActorFromClass` (`KismetArrayLibrary.Array_Random` (`self.Spawnable`)) (`KismetMathLibrary.MakeTransform` (`self.GetSpawnLoc` (`self.Enemy4`))) "AlwaysSpawn" "OverrideRootScale" null null)
    (`|SpawnActorFromClass` (`KismetArrayLibrary.Array_Random` (`self.Spawnable`)) (`KismetMathLibrary.MakeTransform` (`self.GetSpawnLoc` (`self.Enemy5`))) "AlwaysSpawn" "OverrideRootScale" null null)
    (`|SpawnActorFromClass` (`KismetArrayLibrary.Array_Random` (`self.Spawnable`)) (`KismetMathLibrary.MakeTransform` (`self.GetSpawnLoc` (`self.Enemy7`))) "AlwaysSpawn" "OverrideRootScale" null null)
    (`|SpawnActorFromClass` (`KismetArrayLibrary.Array_Random` (`self.Spawnable`)) (`KismetMathLibrary.MakeTransform` (`self.GetSpawnLoc` (`self.Enemy6`))) "AlwaysSpawn" "OverrideRootScale" null null)
    (`|SpawnActorFromClass` (`KismetArrayLibrary.Array_Random` (`self.Spawnable`)) (`KismetMathLibrary.MakeTransform` (`self.GetSpawnLoc` (`self.Enemy1`))) "AlwaysSpawn" "OverrideRootScale" null null)
    (`|SpawnActorFromClass` (`KismetArrayLibrary.Array_Random` (`self.Spawnable`)) (`KismetMathLibrary.MakeTransform` (`self.GetSpawnLoc` (`self.Enemy2`))) "AlwaysSpawn" "OverrideRootScale" null null)
    (`|SpawnActorFromClass` (`KismetArrayLibrary.Array_Random` (`self.Spawnable`)) (`KismetMathLibrary.MakeTransform` (`self.GetSpawnLoc` (`self.Enemy3`))) "AlwaysSpawn" "OverrideRootScale" null null)
    (`|SpawnActorFromClass` (`KismetArrayLibrary.Array_Random` (`self.Pickups`)) (`KismetMathLibrary.MakeTransform` (`self.GetSpawnLoc` (`self.Pickup1`))) "AlwaysSpawn" "OverrideRootScale" null null)
    (`|SpawnActorFromClass` (`KismetArrayLibrary.Array_Random` (`self.Pickups`)) (`KismetMathLibrary.MakeTransform` (`self.GetSpawnLoc` (`self.Pickup2`))) "AlwaysSpawn" "OverrideRootScale" null null)))

(fn `UserConstructionScript`)