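; BP_Top is the top-of-climb environment actor that detects when PlayerRoot reaches it and can populate itself with random content.
; On BeginPlay, if Make is set, it spawns random Spawnable classes at eight scene-component markers and random Pickups at two more.
; When PlayerRoot enters its Box, it fires the player's OnReachTop dispatcher and spawns a B_Flower at the player's location.
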(event `self.ReceiveBeginPlay`
  (bind _outitem (`KismetArrayLibrary.Array_Random` (`self.Spawnable`)))
  (bind _returnvalue (`GameplayStatics.GetActorOfClass` "/Script/RootsGGJ23.PlayerRoot"))
  (set `self.Player` _returnvalue)
  (if (`self.make`)
    (`|SpawnActorFromClass` _outitem (`KismetMathLibrary.MakeTransform` (`SceneComponent.K2_GetComponentLocation` (`self.Scene`))) "AlwaysSpawn" "OverrideRootScale" null null)
    (`|SpawnActorFromClass` _outitem (`KismetMathLibrary.MakeTransform` (`SceneComponent.K2_GetComponentLocation` (`self.Scene6`))) "AlwaysSpawn" "OverrideRootScale" null null)
    (`|SpawnActorFromClass` _outitem (`KismetMathLibrary.MakeTransform` (`SceneComponent.K2_GetComponentLocation` (`self.Scene5`))) "AlwaysSpawn" "OverrideRootScale" null null)
    (`|SpawnActorFromClass` _outitem (`KismetMathLibrary.MakeTransform` (`SceneComponent.K2_GetComponentLocation` (`self.Scene4`))) "AlwaysSpawn" "OverrideRootScale" null null)
    (`|SpawnActorFromClass` _outitem (`KismetMathLibrary.MakeTransform` (`SceneComponent.K2_GetComponentLocation` (`self.Scene3`))) "AlwaysSpawn" "OverrideRootScale" null null)
    (`|SpawnActorFromClass` _outitem (`KismetMathLibrary.MakeTransform` (`SceneComponent.K2_GetComponentLocation` (`self.Scene2`))) "AlwaysSpawn" "OverrideRootScale" null null)
    (`|SpawnActorFromClass` _outitem (`KismetMathLibrary.MakeTransform` (`SceneComponent.K2_GetComponentLocation` (`self.Scene1`))) "AlwaysSpawn" "OverrideRootScale" null null)
    (`|SpawnActorFromClass` _outitem (`KismetMathLibrary.MakeTransform` (`SceneComponent.K2_GetComponentLocation` (`self.Scene7`))) "AlwaysSpawn" "OverrideRootScale" null null)
    (`|SpawnActorFromClass` (`KismetArrayLibrary.Array_Random` (`self.Pickups`)) (`KismetMathLibrary.MakeTransform` (`SceneComponent.K2_GetComponentLocation` (`self.Scene9`))) "AlwaysSpawn" "OverrideRootScale" null null)
    (`|SpawnActorFromClass` (`KismetArrayLibrary.Array_Random` (`self.Pickups`)) (`KismetMathLibrary.MakeTransform` (`SceneComponent.K2_GetComponentLocation` (`self.Scene8`))) "AlwaysSpawn" "OverrideRootScale" null null)))

(event `self.Box.OnComponentBeginOverlap`
  (params (OverlappedComponent :type "PrimitiveComponent Object Reference") (OtherActor :type "Actor Object Reference") (OtherComp :type "PrimitiveComponent Object Reference") (OtherBodyIndex :type Integer) (bFromSweep :type Boolean) (SweepResult :type "HitResult Structure (by ref)"))
  (bind _asplayer_root (cast `PlayerRoot` OtherActor))
  (`PlayerRoot.CallOnReachTop` _asplayer_root)
  (`|SpawnActorFromClass` "/Game/Blueprints/FlowerBuild/B_Flower.B_Flower_C" (`KismetMathLibrary.MakeTransform` (`self.K2_GetActorLocation` _asplayer_root)) "AlwaysSpawn" "OverrideRootScale" null null))

(fn `UserConstructionScript`)