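; BP_Stem is an environment actor that displays a cable as a stem attached to the player.
; On BeginPlay it finds the PlayerRoot actor and binds to its OnStartGrowing event, which makes the Cable component visible.
; Every Tick it teleports to the player's Y and Z at a fixed X and copies the player's rotation.
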(event `self.ReceiveBeginPlay`
  (bind _returnvalue (`GameplayStatics.GetActorOfClass` "/Script/RootsGGJ23.PlayerRoot"))
  (bind _output_get (set `self.Player` _returnvalue))
  (add `PlayerRoot.OnStartGrowing` _output_get (delegate `CustomEvent`)))

(event `CustomEvent`
  (`SceneComponent.SetVisibility` (`self.Cable`) true false))

(event `self.ReceiveTick`
  (params (DeltaSeconds :type "Float (single-precision)"))
  (bind _player (`self.Player`))
  (bind (_returnvalue_x _returnvalue_y _returnvalue_z) (`KismetMathLibrary.BreakVector` (`self.K2_GetActorLocation` _player)))
  (`self.K2_SetActorLocation` (`KismetMathLibrary.MakeVector` 4.0 _returnvalue_y _returnvalue_z) false true)
  (`self.K2_SetActorRotation` (`self.K2_GetActorRotation` _player)))

(fn `UserConstructionScript`)