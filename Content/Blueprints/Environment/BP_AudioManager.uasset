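; BP_AudioManager is an environment audio actor that starts a sound with a fade when the player begins growing.
; On BeginPlay it finds the PlayerRoot actor and binds to its OnStartGrowing event.
; When that fires, it plays its Sound asset at zero volume, then a timeline drives the volume multiplier.
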(event `self.ReceiveBeginPlay`
  (bind _returnvalue (`GameplayStatics.GetActorOfClass` "/Script/RootsGGJ23.PlayerRoot"))
  (bind _output_get (set `self.Player` _returnvalue))
  (`/Engine/EditorBlueprintResources/StandardMacros.IsValid` _output_get
    (:`Is Valid`
      (add `PlayerRoot.OnStartGrowing` _output_get (delegate `OnStartGrowing`)))))

(event `OnStartGrowing`
  (bind _audio (`self.Audio`))
  (`AudioComponent.SetVolumeMultiplier` _audio 0.0)
  (`AudioComponent.SetSound` _audio (`self.Sound`))
  (`AudioComponent.Play` _audio 0.0)
  (bind (_direction _newtrack_0) (`Timeline|Timeline_0` :!via `PlayFromStart`)
    (:`Update`
      (`AudioComponent.SetVolumeMultiplier` _audio _newtrack_0))))

(fn `UserConstructionScript`)