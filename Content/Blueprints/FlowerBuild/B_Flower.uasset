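; B_Flower is a flower actor that stops the player on box overlap and grows a flower from their approach.
; On overlap it zeroes the player's speeds, sends WorldHappiness to B_OverWorldEffect, and builds a spline from recent path points and player position.
; A fourth point extends along the player's up vector, scaled by pre-impact current speed and MaxDistance, where a Paper2D flipbook face spawns.
; BuildStemOfFlower is an empty stub.
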(event `self.Box.OnComponentBeginOverlap`
  (params (OverlappedComponent :type "PrimitiveComponent Object Reference") (OtherActor :type "Actor Object Reference") (OtherComp :type "PrimitiveComponent Object Reference") (OtherBodyIndex :type Integer) (bFromSweep :type Boolean) (SweepResult :type "HitResult Structure (by ref)"))
  (bind _asplayer_root (cast `PlayerRoot` OtherActor))
  (bind _output_get (set `self.HolderMSpeed` (`PlayerRoot.MaxSpeed` _asplayer_root)))
  (bind _output_get_2 (set `self.HolderCSpeed` (`PlayerRoot.CurrentSpeed` _asplayer_root)))
  (set `PlayerRoot.MaxSpeed` 0.0 _asplayer_root)
  (set `PlayerRoot.CurrentSpeed` 0.0 _asplayer_root)
  (bind _returnvalue (`GameplayStatics.GetActorOfClass` "/Game/PostProssessing/B_OverWorldEffect.B_OverWorldEffect_C"))
  (message `/Game/PostProssessing/BI_HitSurface.HitSurface` _returnvalue (`self.World Happiness`))
  (`self.BuildImpactPoints` OtherActor)
  (`self.BuildFlowerLines` OtherActor _output_get _output_get_2)
  (`self.BuildFlowerFace`))

(fn `BuildFlowerFace`
  ;[1 1 1] This is the information where you place the Flowers Face
  (bind _returnvalue (`AddComponent|NODE_AddPaperFlipbookComponent-2` :`RelativeTransform` (`KismetMathLibrary.MakeTransform` (`SplineComponent.GetLocationAtSplinePoint` (`self.Spline`) 3 "Local") (struct) (0.1 1.0 0.1))))
  (`PaperFlipbookComponent.SetFlipbook` _returnvalue "/Game/Assets/IMG.IMG"))

(fn `BuildFlowerLines`
  (params (PlayerActor :type "Actor Object Reference") (MaxSpeed :type "Float (double-precision)") (CurrentSpeed :type "Float (double-precision)"))
  (bind _asplayer_root (cast `PlayerRoot` PlayerActor))
  (`KismetSystemLibrary.PrintString` (`KismetTextLibrary.Conv_TextToString` (`|FormatText` "MAX :: {M} \nCURRENT :: {C}" MaxSpeed CurrentSpeed)))
  (bind _returnvalue (+ (`self.K2_GetActorLocation` _asplayer_root) (* (`self.GetActorUpVector` _asplayer_root) (`KismetMathLibrary.Lerp` CurrentSpeed MaxSpeed 0.0) (`self.MaxDistance`))))
  (`KismetArrayLibrary.Array_Set` (`self.impactPoint`) 3 _returnvalue true)
  (`SplineComponent.AddSplinePointAtIndex` (`self.Spline`) _returnvalue 3 "World" true))

(fn `BuildImpactPoints`
  (params (GetActor :type "Actor Object Reference"))
  (bind _impactpoint (`self.impactPoint`))
  (bind _asplayer_root (cast `PlayerRoot` GetActor))
  (bind _pathpoints (`PlayerRoot.PathPoints` _asplayer_root))
  (bind _returnvalue (`KismetArrayLibrary.Array_LastIndex` _pathpoints))
  (`KismetArrayLibrary.Array_Set` _impactpoint 0 (`|GetArrayItem` _pathpoints (- _returnvalue 1)) true)
  (`KismetArrayLibrary.Array_Set` _impactpoint 1 (`|GetArrayItem` _pathpoints _returnvalue) true)
  (`KismetArrayLibrary.Array_Set` _impactpoint 2 (`self.K2_GetActorLocation` _asplayer_root) true)
  (`SplineComponent.SetSplinePoints` (`self.Spline`) (`self.impactPoint`) "World" true))

(fn `BuildStemOfFlower`)

(fn `UserConstructionScript`)